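; BP_Triviador_Character is the player character for the Triviador game, letting the player pick map tiles by mouse click.
; On BeginPlay it activates its camera and caches the player name from BP_Triviador_PC.
; A left click traces under the cursor; hitting exactly a BP_Country_Part_Base sets TileIsChosen on BP_Triviador_PS and has the tile change color using that state's color and player name.
; All lookups use player controller 0.
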(event Custom|What%20Clicked
  (bind _returnvalue (Game|GetPlayerController 0))
  (bind _hitresult (Game|Player|GetHitResultUnderCursorbyChannel _returnvalue "TraceTypeQuery1" true))
  (bind _playerstate (Variables|/Script/Engine.Controller|GetPlayerState _returnvalue))
  (bind (_bblockinghit _binitialoverlap _time _distance _location _impactpoint _normal _impactnormal _physmat _hitactor) (Collision|BreakHitResult _hitresult))
  (bind _asbp_triviador_ps (Utilities|Casting|CastToBP_Triviador_PS _playerstate))
  (if _bblockinghit
    (if (== (Utilities|GetClass _hitactor) "/Game/-Triviador/Blueprints/Objects/BP_Country_Part_Base.BP_Country_Part_Base_C")
      (Variables|/Game/-Triviador/Blueprints/Player/BP_Triviador_PS.BP_Triviador_PS_C|SettileIsChosen _asbp_triviador_ps true)
      (Default|CallChangeColor (.AsBP%20Country%20Part%20Base (Utilities|Casting|CastToBP_Country_Part_Base _hitactor)) (Variables|/Game/-Triviador/Blueprints/Player/BP_Triviador_PS.BP_Triviador_PS_C|GetE_Color _asbp_triviador_ps) (Variables|Default|GetName) _asbp_triviador_ps)
      (else
        (Development|PrintString "Hello")))))

(event Collision|EventActorBeginOverlap
  (params (OtherActor :type Actor%20Object%20Reference)))

(event EventTick
  (params (DeltaSeconds :type Float%20%28single-precision%29)))

(event EventBeginPlay
  (Components|Activation|Activate (Variables|Default|GetCamera) false)
  (Variables|Default|SetName (Variables|/Game/-Triviador/Blueprints/Player/BP_Triviador_PC.BP_Triviador_PC_C|GetPlayer%20Name (.AsBP%20Triviador%20PC (Utilities|Casting|CastToBP_Triviador_PC (Game|GetPlayerController 0))))))

(event Input|MouseEvents|LeftMouseButton
  (params (Key :type Key%20Structure :default "None"))
  (:Pressed
    (CallFunction|WhatClicked)))

(fn ConstructionScript)