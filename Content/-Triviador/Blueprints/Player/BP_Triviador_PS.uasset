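; Player state for the Triviador trivia game, holding a player's ID, color and answers to choose questions.
; BeginPlay binds answer events and assigns a color by ID; submitted answers go through a server event that stores them and clears TileIsChosen.
; Sorting collects other players' answers by filtering out its own ID.
; It also opens the choose-question widget for the local controller; the TileIsChosen RepNotify only prints a debug message.
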(event Custom|Choose%20Answer
  (params (Answer :type Integer) (Lin%20Color :type Linear%20Color%20Structure))
  ;[1 1 1] Write Player's Choose Answer
  (CallFunction|ServerUpdateChooseAnswer Answer Lin%20Color))

(event Custom|Server_UpdateChooseAnswer
  (params (Answer :type Integer) (Lin%20Color :type Linear%20Color%20Structure))
  ;[1 1 1] Write Player's Choose Answer
  (Variables|Default|SetCQ_Answer (Utilities|Struct|MakePlayer_Choose_Answer (Variables|Default|GetID) Answer self Lin%20Color))
  (Variables|Default|SettileIsChosen false))

(event Custom|Sort%20Choose%20Answers
  (params (Answers :type Array%20of%20Player%20Choose%20Answer%20Structures))
  ;[1 1 1] Get other players answers from ALL answers array
  (for _array_element Answers
    (if (not (== (.PlayerID (Utilities|Struct|BreakPlayer_Choose_Answer _array_element)) (Variables|Default|GetID)))
      (Utilities|Array|AddUnique (Variables|Default|GetOther_CQ_Answers) _array_element))))

(event Custom|Open%20Choose%20Question%20PS
  ;[1 1 1] Open Choose Question Widget
  (if (Pawn|IsLocalPlayerController (Game|GetPlayerController 0))
    (bind _returnvalue (UserInterface|CreateWidget "/Game/-Triviador/Blueprints/Widgets/W_Choose_Question.W_Choose_Question_C"))
    (UserInterface|Viewport|AddtoViewport _returnvalue 0)
    (bind _output_get (Variables|/Game/-Triviador/Blueprints/Widgets/W_Choose_Question.W_Choose_Question_C|SetPS%20Owner _returnvalue self))
    (Default|SetandPrintOwner _returnvalue)
    (Variables|Default|SetCurrent%20Widget%20Choose%20Question _returnvalue)))

(event Custom|Show%20Choose%20Answers
  ;[1 1 1] Show Choose Question Answers
  (Default|ShowAnswers (Variables|Default|GetCurrent%20Widget%20Choose%20Question))
  (Utilities|FlowControl|Delay 3.0))

(event Custom|Print%20Info
  (Development|PrintString (Utilities|String|ToString(Integer) (Variables|Default|GetID))))

(event EventBeginPlay
  (EventDispatchers|BindEventtoSortAnswers (delegate Custom|Sort%20Choose%20Answers))
  (EventDispatchers|BindEventtoUpdateChooseAnswer (delegate Custom|Choose%20Answer))
  (switch int (Variables|Default|GetID)
    (:1
      (Variables|Default|SetE_Color "NewEnumerator0"))
    (:2
      (Variables|Default|SetE_Color "NewEnumerator1"))
    (:3
      (Variables|Default|SetE_Color "NewEnumerator2"))
    (:4
      (Variables|Default|SetColor "(R=1.000000,G=0.000000,B=0.824260,A=1.000000)"))
    (:5
      (Variables|Default|SetColor "(R=0.000000,G=1.000000,B=0.862068,A=1.000000)"))
    (:6
      (Variables|Default|SetColor "(R=0.214954,G=0.000000,B=1.000000,A=1.000000)"))))

(event EventTick
  (params (DeltaSeconds :type Float%20%28single-precision%29)))

(fn ConstructionScript)

(fn OnRepTileIsChosen
  (Development|PrintString "BONG!" true true (Variables|Default|GetColor)))