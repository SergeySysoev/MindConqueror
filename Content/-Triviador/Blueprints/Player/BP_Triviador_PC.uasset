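; Player controller for the Triviador game, handling a player's connection announcement and territory claims on the country map.
; After a short delay on BeginPlay, it sends its PlayerID to all actors implementing the connected-to-game interface.
; Claimed country parts are recorded in Territory by pick order: the first becomes a castle, later ones are recolored and broadcast through the tile-chosen interface.
; It also creates the countdown widget; the tile-chosen OnRep is empty.
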(event Custom|Print%20Info
  (Development|PrintString (Utilities|String|ToString(Integer) (Variables|Default|GetPlayer%20ID))))

(event Custom|PC_ChangeCountryColor
  (params (Country%20Part :type BP%20Country%20Part%20Base%20Object%20Reference) (Color :type E_Player_Color%20Enum :default "NewEnumerator0"))
  ;[1 1 1] Change color of BP Country part
  (if (== (Variables|Default|GetLast%20chosen%20tile) 0)
    (Utilities|Map|Add (Variables|Default|GetTerritory) Country%20Part 0)
    (Variables|Default|SetLast%20chosen%20tile (+ (Variables|Default|GetLast%20chosen%20tile) 1))
    (Default|SCSetCastle Country%20Part Color (Variables|Default|GetPlayer%20ID))
    (else
      (Utilities|Map|Add (Variables|Default|GetTerritory) Country%20Part (Variables|Default|GetLast%20chosen%20tile))
      (Variables|Default|SetLast%20chosen%20tile (+ (Variables|Default|GetLast%20chosen%20tile) 1))
      (Default|SCChangeColor Country%20Part Color (Variables|Default|GetPlayer%20ID))
      (bind _outactors (Actor|GetAllActorswithInterface "/Game/-Triviador/Blueprints/Core/BP_I_TileIsChosen.BP_I_TileIsChosen_C"))
      (for _array_element _outactors
        (Class|BPITileIsChosen|TileIsChosen(Message) _array_element (Variables|Default|GetPlayer%20ID))))))

(event Custom|Show%20Countdown
  (bind _returnvalue (UserInterface|CreateWidget "/Game/-Triviador/Blueprints/Widgets/W_CountdownTimer.W_CountdownTimer_C"))
  (UserInterface|Viewport|AddtoViewport _returnvalue 0))

(event EventBeginPlay
  (Utilities|FlowControl|Delay 4.0)
  (bind _outactors (Actor|GetAllActorswithInterface "/Game/-Triviador/Blueprints/Core/BP_I_ConnectedToGame.BP_I_ConnectedToGame_C"))
  (for _array_element _outactors
    (Class|BPIConnectedtoGame|ConnectedtoGame(Message) _array_element (Variables|Default|GetPlayer%20ID))))

(event EventTick
  (params (DeltaSeconds :type Float%20%28single-precision%29)))

(event Input|KeyboardEvents|P
  (params (Key :type Key%20Structure :default "None")))

(fn ConstructionScript)

(fn OnRepTileIsChose)