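; Game mode for the Triviador multiplayer trivia game, running player setup and the choose-question round on the server.
; On login it assigns IDs and names, then spawns and possesses a character per player.
; Once every player has chosen a tile, each PlayerState opens its question widget.
; Fixed timers from BeginPlay, independent of readiness, tick a countdown, gather PlayerState answers, then send them back through each PlayerState for sorting.
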(event Custom|Server%20Update%20Answers
  ;[1 1 1] Server Update Answers
  (for _array_element (Variables|/Script/Engine.GameStateBase|GetPlayerArray (.AsBP%20Triviador%20GS (Utilities|Casting|CastToBP_Triviador_GS (Game|GetGameState))))
    (bind _asbp_triviador_ps (Utilities|Casting|CastToBP_Triviador_PS _array_element)
      (:then
        (Utilities|Array|Add (Variables|Default|GetPlayers%20Choose%20Answers) (Variables|/Game/-Triviador/Blueprints/Player/BP_Triviador_PS.BP_Triviador_PS_C|GetCQ_Answer _asbp_triviador_ps)))
      (:CastFailed
        (Development|PrintString "cast to PS failed"))))
  (CallFunction|PrintChooseAnswers))

(event Custom|Update%20C%20Answers
  (CallFunction|ServerUpdateAnswers))

(event Custom|Show%20Answers
  (CallFunction|TransferAnswerstoClients))

(event Custom|Transfer%20Answers%20to%20Clients
  ;[1 1 1] Transfer Answers to All clients
  (for _array_element (Variables|/Script/Engine.GameStateBase|GetPlayerArray (.AsBP%20Triviador%20GS (Utilities|Casting|CastToBP_Triviador_GS (Game|GetGameState))))
    (bind _asbp_triviador_ps (Utilities|Casting|CastToBP_Triviador_PS _array_element))
    (Default|CallSortAnswers _asbp_triviador_ps (Variables|Default|GetPlayers%20Choose%20Answers))))

(event Custom|Server%20Countdown%20Timer
  ;[1 1 1] Servet Timer to choose question
  (if (not (== (Variables|Default|GetSeconds) 0))
    (Variables|Default|SetSeconds (- (Variables|Default|GetSeconds) 1))))

(event Custom|Countdown
  (CallFunction|ServerCountdownTimer))

(event EventBeginPlay
  ;[1 1 1] Begin Play
  (Utilities|Time|SetTimerbyEvent (delegate Custom|Update%20C%20Answers) 1e+01)
  (Utilities|Time|SetTimerbyEvent (delegate Custom|Show%20Answers) 11.0)
  (Utilities|Time|SetTimerbyEvent (delegate Custom|Countdown) 1.0 true))

(event EventTick
  (params (DeltaSeconds :type Float%20%28single-precision%29)))

(event EventPostLogin
  (params (NewPlayer :type Player%20Controller%20Object%20Reference))
  ;[1 1 1] Post Login
  (Utilities|Array|AddUnique (Variables|Default|GetPlayer%20Controllers) NewPlayer)
  (bind _asbp_triviador_pc (Utilities|Casting|CastToBP_Triviador_PC NewPlayer))
  (Variables|/Game/-Triviador/Blueprints/Player/BP_Triviador_PC.BP_Triviador_PC_C|SetPlayer%20ID _asbp_triviador_pc (Variables|Default|GetNext%20Player%20ID))
  (bind _asbp_triviador_ps (Utilities|Casting|CastToBP_Triviador_PS (Variables|/Script/Engine.Controller|GetPlayerState _asbp_triviador_pc)))
  (Variables|/Game/-Triviador/Blueprints/Player/BP_Triviador_PS.BP_Triviador_PS_C|SetID _asbp_triviador_ps (Variables|Default|GetNext%20Player%20ID))
  (Variables|/Game/-Triviador/Blueprints/Player/BP_Triviador_PC.BP_Triviador_PC_C|SetReady%20to%20Play _asbp_triviador_pc true)
  (Variables|/Game/-Triviador/Blueprints/Player/BP_Triviador_PC.BP_Triviador_PC_C|SetPlayer%20Name _asbp_triviador_pc (Utilities|Array|Get(acopy) (Variables|Default|GetPlayer%20Names) (- (Variables|Default|GetNext%20Player%20ID) 1)))
  (Utilities|Array|Add (Variables|Default|GetPlayers%20Ready) false)
  (Variables|Default|SetNext%20Player%20ID (+ (Variables|Default|GetNext%20Player%20ID) 1)))

(event EventHandleStartingNewPlayer
  (params (NewPlayer :type Player%20Controller%20Object%20Reference))
  (Networking|SwitchHasAuthority
    (:Authority
      (bind _returnvalue (Game|SpawnActorfromClass "/Game/-Triviador/Blueprints/Player/BP_Triviador_Character.BP_Triviador_Character_C" (Transformation|GetActorTransform (Class|GameModeBase|FindPlayerStart NewPlayer)) "AdjustIfPossibleButAlwaysSpawn" NewPlayer 0))
      (Pawn|Possess NewPlayer _returnvalue)
      (Development|PrintString (Utilities|String|Append "Player connected:   " (Utilities|GetDisplayName NewPlayer))))))

(event EventTileIsChosen
  (params (PlayerID :type Integer))
  (bind _players_ready (Variables|Default|GetPlayers%20Ready))
  ;[1 1 1] Check whether all players are ready or not
  ; If yes, open their Choose Question Widget
  (Utilities|Array|SetArrayElem _players_ready PlayerID true)
  (if (not (Utilities|Array|ContainsItem _players_ready false))
    (for _array_element (Variables|/Script/Engine.GameStateBase|GetPlayerArray (.AsBP%20Triviador%20GS (Utilities|Casting|CastToBP_Triviador_GS (Game|GetGameState))))
      (bind _asbp_triviador_ps (Utilities|Casting|CastToBP_Triviador_PS _array_element))
      (Default|ClientOpenChooseQuestion _asbp_triviador_ps))))

(fn ConstructionScript)

(fn PrintChooseAnswers
  (for _array_element (Variables|Default|GetPlayers%20Choose%20Answers)
    (Development|PrintString (Utilities|String|Append (Utilities|String|ToString(Integer) (.PlayerID (Utilities|Struct|BreakPlayer_Choose_Answer _array_element))) "------" (Utilities|String|ToString(Integer) (.Answer (Utilities|Struct|BreakPlayer_Choose_Answer _array_element))) "-" (Utilities|String|ToString(Integer) (.Color (Utilities|Struct|BreakPlayer_Choose_Answer _array_element)))) true true (.Color (Utilities|Struct|BreakPlayer_Choose_Answer _array_element)))))