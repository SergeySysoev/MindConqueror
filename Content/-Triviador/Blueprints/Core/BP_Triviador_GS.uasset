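; BP_Triviador_GS, apparently the Game State for the Triviador game, tracks which players are ready.
; On BeginPlay it binds a handler to a player-ready event, which flags that player's ID in the PlayersReady array, ignoring repeats.
; Once no entry is false it only prints the game mode's display name, with no further game flow triggered.
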(event Custom|Update%20PlayerReady%20Array
  (params (PlayerID :type Integer))
  (bind _players_ready (Variables|Default|GetPlayers%20Ready))
  (if (not (Utilities|Array|Get(acopy) _players_ready PlayerID))
    (Utilities|Array|SetArrayElem _players_ready PlayerID true)
    (if (not (Utilities|Array|ContainsItem (Variables|Default|GetPlayers%20Ready) false))
      (Development|PrintString (Utilities|GetDisplayName (Game|GetGameMode))))))

(event EventBeginPlay
  (EventDispatchers|BindEventtoPlayerReady (delegate Custom|Update%20PlayerReady%20Array)))

(event EventTick
  (params (DeltaSeconds :type Float%20%28single-precision%29)))

(fn ConstructionScript)