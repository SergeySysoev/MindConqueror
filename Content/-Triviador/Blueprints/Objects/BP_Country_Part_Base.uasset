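; Base actor for a country tile on the Triviador map that players can claim or turn into a castle.
; Color requests route through BP_Triviador_PC, and SC_ events store owner color, player ID and castle state.
; RepNotifies then color the sphere marker for claimed tiles or the tile mesh for castles.
; A sphere trace gathers neighboring tiles, which are recolored through the player controller; hover highlighting is disconnected.
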(event OnBeginCursorOver(StaticMesh)
  (params (TouchedComponent :type Primitive%20Component%20Object%20Reference))
  ;[1 1 1] Highlight a block on cursor over
)

(event OnEndCursorOver(StaticMesh)
  (params (TouchedComponent :type Primitive%20Component%20Object%20Reference))
  ;[1 1 1] Highlight a block on cursor over
)

(event Custom|SC_SetCastle
  (params (Color :type E_Player_Color%20Enum :default "NewEnumerator0") (Player%20ID :type Integer))
  ;[1 1 1] Change color of a Tile
  (bind _output_get (Variables|Default|SetOwnerColor Color))
  (Variables|Default|SetClickedPlayerID Player%20ID)
  (Rendering|SetVisibility (Variables|Default|GetBillboard) true false)
  (Variables|Default|SetCasteIsChosen true)
  (CallFunction|SetMaterialOfStaticMesh (Variables|Default|GetStaticMesh) _output_get false)
  (Variables|Default|SethasOwner true)
  (Variables|Default|SetisCastle true))

(event Custom|SC_ChangeColor
  (params (Color :type E_Player_Color%20Enum :default "NewEnumerator0") (PlayerID :type Integer))
  ;[1 1 1] Change color of a Tile
  (Variables|Default|SetOwnerColor Color)
  (Variables|Default|SetClickedPlayerID PlayerID)
  (Variables|Default|SetisPressed true)
  (Variables|Default|SethasOwner true))

(event Custom|Set%20the%20color
  (params (Player%20Color :type E_Player_Color%20Enum :default "NewEnumerator0"))
  ;[1 1 1] Change color of a Tile
  (if (and (not (Variables|Default|GetisCastle)) (not (Variables|Default|GethasOwner)))
    (if (not (Variables|Default|GetisPressed))
      (bind _output_get (Variables|Default|SetOwnerColor Player%20Color))
      (Development|PrintString (Utilities|String|Append "" "------" (Utilities|GetObjectName 0) "------" (Utilities|String|EnumtoString _output_get)))
      (Default|PCChangeCountryColor (.AsBP%20Triviador%20PC (Utilities|Casting|CastToBP_Triviador_PC (Game|GetPlayerController 0))) self (Variables|Default|GetOwnerColor)))))

(event Custom|Set%20Color%20for%20the%20Nearest%20Country%20Parts
  (params (Color :type E_Player_Color%20Enum :default "NewEnumerator0"))
  (Default|PCChangeColorOftheNearestCountryParts (.AsBP%20Triviador%20PC (Utilities|Casting|CastToBP_Triviador_PC (Game|GetPlayerController 0))) self Color))

(event Custom|CC%20Change%20Color%20of%20the%20Nearest%20Country%20Parts
  (params (Color :type E_Player_Color%20Enum :default "NewEnumerator0") (Player%20ID :type Integer))
  (Variables|Default|SetClickedPlayerID Player%20ID)
  (CallFunction|SetMaterialOfStaticMesh (Variables|Default|GetStaticMesh) Color true))

(event EventBeginPlay
  (EventDispatchers|BindEventtoChangeColor (delegate Custom|Set%20the%20color)))

(event EventTick
  (params (DeltaSeconds :type Float%20%28single-precision%29)))

(fn ConstructionScript)

(fn OnRepIsPressed
  (CallFunction|SetMaterialOfStaticMesh (Variables|Default|GetSphere) (Variables|Default|GetOwnerColor) true))

(fn SetMaterialOfStaticMesh
  (params (Static%20Mesh :type Static%20Mesh%20Component%20Object%20Reference) (Color :type E_Player_Color%20Enum :default "NewEnumerator0") (Turn%20Visibility :type Boolean))
  (if Turn%20Visibility
    (Rendering|SetVisibility Static%20Mesh true false))
  (switch Utilities|FlowControl|Switch|SwitchonE_Player_Color Color
    (:NewEnumerator0
      (Rendering|Material|SetMaterial Static%20Mesh 0 "/Game/-Triviador/Materials/MI_TileRed.MI_TileRed"))
    (:NewEnumerator1
      (Rendering|Material|SetMaterial Static%20Mesh 0 "/Game/-Triviador/Materials/MI_TileGreen.MI_TileGreen"))
    (:NewEnumerator2
      (Rendering|Material|SetMaterial Static%20Mesh 0 "/Game/-Triviador/Materials/MI_TileBlue.MI_TileBlue"))
    (:NewEnumerator3
      (Rendering|Material|SetMaterial Static%20Mesh 0 "/Game/-Triviador/Materials/MI_TilePink.MI_TilePink"))
    (:NewEnumerator4
      (Rendering|Material|SetMaterial Static%20Mesh 0 "/Game/-Triviador/Materials/MI_TileCyan.MI_TileCyan"))
    (:NewEnumerator5
      (Rendering|Material|SetMaterial Static%20Mesh 0 "/Game/-Triviador/Materials/MI_TilePurple.MI_TilePurple"))))

(fn OnRepCasteIsChosen
  (CallFunction|SetMaterialOfStaticMesh (Variables|Default|GetStaticMesh) (Variables|Default|GetOwnerColor) false))

(fn FindNearestCountryParts
  (params (Color :type E_Player_Color%20Enum :default "NewEnumerator0"))
  (bind _returnvalue (Transformation|GetActorLocation))
  (bind _nearparts (Variables|Default|GetNearParts))
  (bind _outhits (Collision|MultiSphereTraceForObjects _returnvalue (+ _returnvalue "0, 0,0.100000") 2e+02 (Utilities|Array|MakeArray "ObjectTypeQuery7") false 0 "ForDuration" true "(R=1.000000,G=0.000000,B=0.000000,A=1.000000)" "(R=0.000000,G=1.000000,B=0.000000,A=1.000000)" 5e+01))
  (for _array_element _outhits
    (Utilities|IsValid (.AsBP%20Country%20Part%20Base (Utilities|Casting|CastToBP_Country_Part_Base (.HitActor (Collision|BreakHitResult _array_element))))
      (:Is%20Valid
        (if (not (Utilities|Array|ContainsItem _nearparts (.AsBP%20Country%20Part%20Base (Utilities|Casting|CastToBP_Country_Part_Base (.HitActor (Collision|BreakHitResult _array_element))))))
          (Utilities|Array|AddUnique _nearparts (.AsBP%20Country%20Part%20Base (Utilities|Casting|CastToBP_Country_Part_Base (.HitActor (Collision|BreakHitResult _array_element)))))))))
  (CallFunction|LighttheNearestCountryParts Color)
  (return))

(fn LighttheNearestCountryParts
  (params (Color :type E_Player_Color%20Enum :default "NewEnumerator0"))
  (for _array_element (Variables|Default|GetNearParts)
    (CallFunction|SetColorfortheNearestCountryParts _array_element Color)))